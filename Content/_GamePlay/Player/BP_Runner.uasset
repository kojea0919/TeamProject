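; BP_Runner is the runner player Blueprint, handling camera zoom and detection of interactable objects.
; On BeginPlay it links the runner animation layer to the mesh and adds an interact-dot widget to the viewport.
; Each Tick it traces from the camera, reads the hit actor's tag and object through message calls, and registers them with RunnerInterActiveComponent.
; Aim and crouch events play or reverse timelines that lerp spring arm length and socket offset.
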(event `self.ReceiveBeginPlay`
  (`|ExecutionSequence`
    (:`then_0`
      (`SkeletalMeshComponent.LinkAnimClassLayers` (`self.Mesh`) "/Game/_GamePlay/Player/Animation/AnimBlueprint/ABP_RunnerLayer.ABP_RunnerLayer_C"))
    (:`then_1`
      (bind _returnvalue (`|CreateWidget` "/Game/_GamePlay/Player/UI/InteractDotWidget.InteractDotWidget_C"))
      (bind _output_get (set `self.InterActDot` _returnvalue))
      (`UserWidget.AddToViewport` _output_get 0))))

(event `self.ReceiveTick`
  (params (DeltaSeconds :type "Float (single-precision)"))
  (bind _camera (`self.Camera`))
  (bind _returnvalue (`SceneComponent.K2_GetComponentLocation` _camera))
  (bind (_outhit _returnvalue_2) (`KismetSystemLibrary.LineTraceSingle` _returnvalue (+ _returnvalue (* (`SceneComponent.GetForwardVector` _camera) 700.0)) "TraceTypeQuery1"))
  (if _returnvalue_2
    (bind (_bblockinghit _binitialoverlap _time _distance _location _impactpoint _normal _impactnormal _physmat _hitactor) (`GameplayStatics.BreakHitResult` _outhit))
    (bind _returnvalue_3 (message `InterActiveInterface.GetObjectTag` _hitactor))
    (bind _returnvalue_4 (message `InterActiveInterface.GetObject` _hitactor))
    (`PawnInterActiveComponent.RegisterSpawnObject` (`self.RunnerInterActiveComponent`) _returnvalue_3 _returnvalue_4 false)))

(event `AimCamera`
  (bind (_direction _arm_lengthdistance) (`Timeline|ZoomCamera` :!label _label)
    (:`Update`
      (set `SpringArmComponent.TargetArmLength` (`KismetMathLibrary.Lerp` 300.0 150.0 _arm_lengthdistance) (`self.SpringArm`))
      (set `SpringArmComponent.SocketOffset` (`KismetMathLibrary.MakeVector` 0.0 (`KismetMathLibrary.Lerp` 0.0 -10.0 _arm_lengthdistance) (`KismetMathLibrary.Lerp` 0.0 0.0 _arm_lengthdistance)) (`self.SpringArm`)))))

(event `AimCameraEnd`
  (goto _label :!via `Reverse`))

(event `CrounchCamera`
  (bind (_direction _arm_lengthdistance) (`Timeline|ZoomCamera2` :!label _label_2)
    (:`Update`
      (set `SpringArmComponent.TargetArmLength` (`KismetMathLibrary.Lerp` 300.0 250.0 _arm_lengthdistance) (`self.SpringArm`))
      (set `SpringArmComponent.SocketOffset` (`KismetMathLibrary.MakeVector` 0.0 0.0 (`KismetMathLibrary.Lerp` 0.0 -70.0 _arm_lengthdistance)) (`self.SpringArm`)))))

(event `CrounchCameraEnd`
  (goto _label_2 :!via `Reverse`))

(fn `UserConstructionScript`)