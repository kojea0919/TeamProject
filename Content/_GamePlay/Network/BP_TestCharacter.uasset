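; Networked test character that adds positional voice chat, a HUD smartphone and widget interaction to the player.
; BeginPlay registers a VOIP talker attached to the camera, retrying until PlayerState is valid, and keeps widget interaction only for the locally controlled authority pawn.
; V toggles speaking and the controller's mic state, Tab animates the phone and switches input mode, Shot clicks widgets.
; Debug leftovers print voice level every tick and fetch a pooled effect on N.
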(event `self.ReceiveBeginPlay`
  (`self.InitializeVoiceChat`)
  (bind _asbp_main_map_player_controller (cast `/Game/_GamePlay/GameFrameWork/MainMap/BP_MainMapPlayerController` (`GameplayStatics.GetPlayerController` 0)))
  (bind _output_get (set `self.IsActiveMic` false))
  (`MainMapPlayerController.SetActiveMic` _asbp_main_map_player_controller _output_get)
  (if (not (and (`self.IsLocallyControlled`) (`self.HasAuthority`)))
    (`ActorComponent.Deactivate` (`self.WidgetInteraction`))))

(event `self.ReceiveTick`
  (params (DeltaSeconds :type "Float (single-precision)"))
  (bind _returnvalue (`VOIPTalker.GetVoiceLevel` (`self.VOIP REF`)))
  (`KismetSystemLibrary.PrintString` (`KismetStringLibrary.Conv_DoubleToString` _returnvalue)))

(event `EnhancedInput|/Game/_GamePlay/Player/Input/IA_Shot`
  (params (ActionValue :type Boolean) (ElapsedSeconds :type "Float (double-precision)") (TriggeredSeconds :type "Float (double-precision)") (InputAction :type "InputAction Object Reference" :default "/Game/_GamePlay/Player/Input/IA_Shot.IA_Shot"))
  (bind _widgetinteraction (`self.WidgetInteraction`))
  (:`Started`
    (`WidgetInteractionComponent.PressPointerKey` _widgetinteraction "LeftMouseButton"))
  (:`Completed`
    (`WidgetInteractionComponent.ReleasePointerKey` _widgetinteraction "LeftMouseButton")))

(event `Key|Tab`
  (params (Key :type "Key Structure"))
  (:`Pressed`
    (`self.SetSmartPhone`)))

(event `Key|N`
  (params (Key :type "Key Structure"))
  (:`Pressed`
    (`self.ClickN`)))

(event `ClickN`
  (`self.CreateExplosion`))

(event `CreateExplosion`
  (bind _returnvalue (`EffectObjectPoolSubSystem.GetEffectObject` (subsystem `EffectObjectPoolSubSystem`) "/Game/_GamePlay/GameFrameWork/Test/BP_TestNiagaraEffect.BP_TestNiagaraEffect_C"))
  (cast `/Game/_GamePlay/GameFrameWork/Test/BP_TestNiagaraEffect` _returnvalue))

(event `InitializeVoiceChat`
  (bind _playerstate (`self.PlayerState`))
  (bind _returnvalue (`AddComponent|NODE_AddVOIPTalker-2`))
  (bind _output_get (set `self.VOIP REF` _returnvalue))
  (`/Engine/EditorBlueprintResources/StandardMacros.IsValid` _playerstate :!label _label
    (:`Is Valid`
      (`VOIPTalker.RegisterWithPlayerState` _output_get _playerstate)
      (`VOIPStatics.SetMicThreshold` -2.0)
      (set `VOIPTalker.Settings` (make `VoiceSettings` (`self.FollowCamera`) "/Game/_GamePlay/VoiceChat/SA_VOIP.SA_VOIP") (`self.VOIP REF`)))
    (:`Is Not Valid`
      (`KismetSystemLibrary.Delay` 0.2)
      (goto _label))))

(event `Key|V`
  (params (Key :type "Key Structure"))
  (:`Pressed`
    (if (`self.IsActiveMic`)
      (bind _asbp_main_map_player_controller (cast `/Game/_GamePlay/GameFrameWork/MainMap/BP_MainMapPlayerController` (`GameplayStatics.GetPlayerController` 0)))
      (bind _output_get (set `self.IsActiveMic` false))
      (`MainMapPlayerController.SetActiveMic` _asbp_main_map_player_controller _output_get)
      (`KismetSystemLibrary.ExecuteConsoleCommand` "ToggleSpeaking 0" null)
      (else
        (bind _asbp_main_map_player_controller_2 (cast `/Game/_GamePlay/GameFrameWork/MainMap/BP_MainMapPlayerController` (`GameplayStatics.GetPlayerController` 0)))
        (bind _output_get_2 (set `self.IsActiveMic` true))
        (`MainMapPlayerController.SetActiveMic` _asbp_main_map_player_controller_2 _output_get_2)
        (`KismetSystemLibrary.ExecuteConsoleCommand` "ToggleSpeaking 1" null)))))

(fn `SetSmartPhone`
  (locals (PlayerController :type "/Game/_GamePlay/GameFrameWork/MainMap/BP_MainMapPlayerController Object Reference"))
  (bind _playercontroller (`local.PlayerController`))
  (bind _playercontroller_2 (`local.PlayerController`))
  (bind _asbp_main_map_player_controller (cast `/Game/_GamePlay/GameFrameWork/MainMap/BP_MainMapPlayerController` (`GameplayStatics.GetPlayerController` 0)))
  (set `local.PlayerController` _asbp_main_map_player_controller)
  (if (`self.IsActivePhone`)
    (bind _playermainhud (`MainMapPlayerController.PlayerMainHUD` _asbp_main_map_player_controller))
    (bind _asw_main_hud (cast `/Game/_GamePlay/UI/MainMapUI/W_MainHud` _playermainhud))
    (`UserWidget.PlayAnimation` _asw_main_hud (`/Game/_GamePlay/UI/MainMapUI/W_MainHud.PutInPhoneAnimation` _asw_main_hud) 0.0 1 "Forward" 1.0 false)
    (set `self.IsActivePhone` false)
    (`WidgetBlueprintLibrary.SetInputMode_GameOnly` _playercontroller)
    (set `PlayerController.bShowMouseCursor` false _playercontroller)
    (else
      (bind _asw_main_hud_2 (cast `/Game/_GamePlay/UI/MainMapUI/W_MainHud` _playermainhud))
      (`UserWidget.PlayAnimation` _asw_main_hud_2 (`/Game/_GamePlay/UI/MainMapUI/W_MainHud.TakeOutPhoneAnimation` _asw_main_hud_2) 0.0 1 "Forward" 1.0 false)
      (set `self.IsActivePhone` true)
      (`WidgetBlueprintLibrary.SetInputMode_UIOnlyEx` _playercontroller_2 _asw_main_hud_2)
      (set `PlayerController.bShowMouseCursor` true _playercontroller_2))))

(fn `UserConstructionScript`)