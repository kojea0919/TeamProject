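; Start map game mode that creates, finds and joins multiplayer Mission sessions through Advanced Sessions nodes.
; Hosting tags the session with a MatchType property and server-travels to MainMap as a listen server.
; Searching filters on that tag, updates the session list and loading image on BP_StartMapPlayerController, and also attempts to join each match immediately.
; Successful joins, including those from the separate JoinSession event, client-travel to the host address.
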(event `self.ReceiveBeginPlay`)

(event `CreateSession`
  (`CreateSessionCallbackProxyAdvanced.CreateAdvancedSession` (`|MakeArray` (`AdvancedSessionsLibrary.MakeLiteralSessionPropertyString` "MatchType" "Mission")) (`GameplayStatics.GetPlayerController` 0) 4 0 false true false true true true false false true true true
    (:`OnSuccess`
      (`AdvancedSessionsLibrary.ServerTravel` "/Game/_GamePlay/Map/MainMap?listen" true))))

(event `JoinSession`
  (params (SessionResult :type "BlueprintSessionResult Structure"))
  (`JoinSessionCallbackProxy.JoinSession` (`GameplayStatics.GetPlayerController` 0) SessionResult
    (:`OnSuccess`
      (bind _returnvalue (`self.GetAddress`))
      (`KismetSystemLibrary.PrintString` _returnvalue)
      (`self.ClientTravel` _returnvalue))
    (:`OnFailure`
      (`KismetSystemLibrary.PrintString` "Fail"))))

(event `FindSession`
  (bind _results (`FindSessionsCallbackProxyAdvanced.FindSessionsAdvanced` (`GameplayStatics.GetPlayerController` 0) 20 false "AllServers" (`|MakeArray` (`AdvancedSessionsLibrary.MakeLiteralSessionSearchProperty` (`AdvancedSessionsLibrary.MakeLiteralSessionPropertyString` "MatchType" "Mission") "Equals")))
    (:`OnSuccess`
      (bind _asbp_start_map_player_controller (cast `/Game/_GamePlay/GameFrameWork/GameStartMap/BP_StartMapPlayerController` (`GameplayStatics.GetPlayerController` 0)))
      (`StartMapPlayerController.SetVisibleSessionLoadImage` _asbp_start_map_player_controller false)
      (bind _asbp_start_map_player_controller_2 (cast `/Game/_GamePlay/GameFrameWork/GameStartMap/BP_StartMapPlayerController` (`GameplayStatics.GetPlayerController` 0))
        (:`then`
          (`StartMapPlayerController.ClearSessionList` _asbp_start_map_player_controller_2)
          (for _array_element _results
            (bind _extrasettings (`AdvancedSessionsLibrary.GetExtraSettings` _array_element))
            (bind _settingvalue (`AdvancedSessionsLibrary.GetSessionPropertyString` _extrasettings "MatchType")
              (:`Found`
                (if (== _settingvalue "Mission")
                  (`StartMapPlayerController.AddToSessionList` _asbp_start_map_player_controller_2 _array_element)
                  (`JoinSessionCallbackProxy.JoinSession` (`GameplayStatics.GetPlayerController` 0) _array_element
                    (:`OnSuccess`
                      (bind _returnvalue (`self.GetAddress`))
                      (`KismetSystemLibrary.PrintString` _returnvalue)
                      (`self.ClientTravel` _returnvalue))
                    (:`OnFailure`
                      (`KismetSystemLibrary.PrintString` "Fail")))))
              (:`NotFound`
                (`KismetSystemLibrary.PrintString` "SessionPropertyString Not Found")))))
        (:`CastFailed`
          (`KismetSystemLibrary.PrintString` "Controller Cast Fail"))))
    (:`OnFailure`
      (bind _asbp_start_map_player_controller_3 (cast `/Game/_GamePlay/GameFrameWork/GameStartMap/BP_StartMapPlayerController` (`GameplayStatics.GetPlayerController` 0)))
      (`StartMapPlayerController.SetVisibleSessionLoadImage` _asbp_start_map_player_controller_3 false)
      (`KismetSystemLibrary.PrintString` "Fail Find Session"))))

(fn `UserConstructionScript`)