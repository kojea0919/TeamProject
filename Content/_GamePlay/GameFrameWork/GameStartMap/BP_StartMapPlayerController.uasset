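; Player controller for the start map that lets the player skip the intro movie by holding Z.
; While Z is held, Tick accumulates time and feeds it to the intro movie widget's square progress indicator.
; Past a one-second hold it calls EndMovie, and releasing Z resets both the timer and the indicator.
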(event `self.ReceiveTick`
  (params (DeltaSeconds :type "Float (single-precision)"))
  (if true
    (if (`self.IsPressSkipKey`)
      (bind _output_get (set `self.AccTime` (+ DeltaSeconds (`self.AccTime`))))
      (if (> _output_get 1.0)
        (`self.EndMovie`)
        (else
          (`IntroMovie.SetSquareProgressTime` (`self.IntroMovieWidget`) _output_get))))))

(event `Key|Z`
  (params (Key :type "Key Structure"))
  (:`Pressed`
    (set `self.IsPressSkipKey` true))
  (:`Released`
    (set `self.IsPressSkipKey` false)
    (set `self.AccTime` 0.0)
    (`IntroMovie.InitSquareProgress` (`self.IntroMovieWidget`))))

(fn `UserConstructionScript`)