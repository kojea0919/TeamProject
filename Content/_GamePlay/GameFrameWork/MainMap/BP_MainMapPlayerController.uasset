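; Player controller for the main map, handling voice chat, the smartphone UI and a few gameplay hotkeys.
; BeginPlay sets up VOIP on the owner cast to Character; V toggles the mic via console command.
; Audio envelope values above a threshold trigger the HUD talking animation.
; Tab animates the phone and switches input mode and cursor, while L calls CheckPrision on GameState and 8 requests ghost mode from GameMode.
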(event `self.ReceiveBeginPlay`
  (bind _ascharacter (cast `Character` (`self.GetOwner`)))
  (bind _returnvalue (`AddComponent|NODE_AddVOIPTalker-0`))
  (`/Game/_GamePlay/VoiceChat/VoiceChatComponent.InitVoiceChat` (`self.VoiceChatComponent`) (`self.PlayerState`) _returnvalue (`Character.Mesh` _ascharacter)))

(event `Key|V`
  (params (Key :type "Key Structure"))
  (:`Pressed`
    (if (`self.IsActiveMic`)
      (bind _asbp_main_map_player_controller (cast `/Game/_GamePlay/GameFrameWork/MainMap/BP_MainMapPlayerController` (`GameplayStatics.GetPlayerController` 0)))
      (bind _output_get (set `self.IsActiveMic` false))
      (`self.SetActiveMic` _asbp_main_map_player_controller _output_get)
      (`KismetSystemLibrary.ExecuteConsoleCommand` "ToggleSpeaking 0" null)
      (else
        (bind _asbp_main_map_player_controller_2 (cast `/Game/_GamePlay/GameFrameWork/MainMap/BP_MainMapPlayerController` (`GameplayStatics.GetPlayerController` 0)))
        (bind _output_get_2 (set `self.IsActiveMic` true))
        (`self.SetActiveMic` _asbp_main_map_player_controller_2 _output_get_2)
        (`KismetSystemLibrary.ExecuteConsoleCommand` "ToggleSpeaking 1" null)))))

(event `Key|Tab`
  (params (Key :type "Key Structure"))
  (:`Pressed`
    (bind _asbp_main_map_game_state (cast `/Game/_GamePlay/GameFrameWork/MainMap/BP_MainMapGameState` (`GameplayStatics.GetGameState`)))
    (`self.SetSmartPhone`)))

(event `self.AudioCapture.OnAudioEnvelopeValue`
  (params (EnvelopeValue :type "Float (single-precision)"))
  (if (and (> EnvelopeValue 0.004) (`KismetSystemLibrary.IsValid` (`self.PlayerMainHUD`)))
    (`PlayerMainHUD.PlayTalkingAnimation` (`self.PlayerMainHUD`))))

(event `Key|L`
  (params (Key :type "Key Structure"))
  (:`Pressed`
    (bind _asbp_main_map_game_state (cast `/Game/_GamePlay/GameFrameWork/MainMap/BP_MainMapGameState` (`GameplayStatics.GetGameState`)))
    (`MainMapGameState.CheckPrision` _asbp_main_map_game_state)))

(event `Key|Eight`
  (params (Key :type "Key Structure"))
  (:`Pressed`
    (`self.ttttt`)))

(event `ttttt`
  (bind _asbp_main_map_game_mode (cast `/Game/_GamePlay/GameFrameWork/MainMap/BP_MainMapGameMode` (`GameplayStatics.GetGameMode`)))
  (bind _asbp_runner (cast `/Game/_GamePlay/Player/BP_Runner` (`GameplayStatics.GetPlayerCharacter` 0)))
  (`MainMapGameMode.SetGhostMode` _asbp_main_map_game_mode _asbp_runner))

(fn `SetSmartPhone`
  (if (`self.IsActivePhone`)
    (bind _asw_main_hud (cast `/Game/_GamePlay/UI/MainMapUI/W_MainHud` (`self.PlayerMainHUD`)))
    (`UserWidget.PlayAnimation` _asw_main_hud (`/Game/_GamePlay/UI/MainMapUI/W_MainHud.PutInPhoneAnimation` _asw_main_hud) 0.0 1 "Forward" 1.0 false)
    (set `self.IsActivePhone` false)
    (`WidgetBlueprintLibrary.SetInputMode_GameOnly` self)
    (set `self.bShowMouseCursor` false)
    (else
      (bind _asw_main_hud_2 (cast `/Game/_GamePlay/UI/MainMapUI/W_MainHud` (`self.PlayerMainHUD`)))
      (`UserWidget.PlayAnimation` _asw_main_hud_2 (`/Game/_GamePlay/UI/MainMapUI/W_MainHud.TakeOutPhoneAnimation` _asw_main_hud_2) 0.0 1 "Forward" 1.0 false)
      (set `self.IsActivePhone` true)
      (`WidgetBlueprintLibrary.SetInputMode_GameAndUIEx` self null)
      (set `self.bShowMouseCursor` true))))

(fn `UserConstructionScript`)