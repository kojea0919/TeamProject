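; Main map game mode that sets up voice chat whenever a player joins.
; PostLogin and HandleStartingNewPlayer run duplicate logic, calling ClientToggleVoiceAtStart on the new controller and then waiting for its pawn.
; It then loops over the PlayerArray and calls MulticastInitVOIP on every player's BP_TestCharacter, not just the newcomer's.
; Missing pawns are polled with short retriggerable delays, including from inside the loop body.
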(event `self.K2_PostLogin`
  (params (NewPlayer :type "PlayerController Object Reference"))
  (`parent.K2_PostLogin` NewPlayer)
  (bind _asbp_main_map_player_controller (cast `/Game/_GamePlay/GameFrameWork/MainMap/BP_MainMapPlayerController` NewPlayer))
  (`/Game/_GamePlay/GameFrameWork/MainMap/BP_MainMapPlayerController.Client_ToggleVoiceAtStart` _asbp_main_map_player_controller)
  (`/Engine/EditorBlueprintResources/StandardMacros.IsValid` (`Controller.K2_GetPawn` _asbp_main_map_player_controller) :!label _label
    (:`Is Valid`
      (for _array_element (`GameStateBase.PlayerArray` (`GameplayStatics.GetGameState`))
        (bind _returnvalue (`Controller.K2_GetPawn` (`PlayerState.GetPlayerController` _array_element)))
        (`/Engine/EditorBlueprintResources/StandardMacros.IsValid` _returnvalue :!label _label_2
          (:`Is Valid`
            (bind _asbp_test_character (cast `/Game/_GamePlay/Network/BP_TestCharacter` _returnvalue))
            (`/Game/_GamePlay/Network/BP_TestCharacter.Multicast_InitVOIP` _asbp_test_character))
          (:`Is Not Valid`
            (`KismetSystemLibrary.RetriggerableDelay` 0.2)
            (goto _label_2)))))
    (:`Is Not Valid`
      (`KismetSystemLibrary.RetriggerableDelay` 0.2)
      (goto _label))))

(event `self.HandleStartingNewPlayer`
  (params (NewPlayer :type "PlayerController Object Reference"))
  (`parent.HandleStartingNewPlayer` NewPlayer)
  (bind _asbp_main_map_player_controller (cast `/Game/_GamePlay/GameFrameWork/MainMap/BP_MainMapPlayerController` NewPlayer))
  (`/Game/_GamePlay/GameFrameWork/MainMap/BP_MainMapPlayerController.Client_ToggleVoiceAtStart` _asbp_main_map_player_controller)
  (`/Engine/EditorBlueprintResources/StandardMacros.IsValid` (`Controller.K2_GetPawn` _asbp_main_map_player_controller) :!label _label_3
    (:`Is Valid`
      (for _array_element (`GameStateBase.PlayerArray` (`GameplayStatics.GetGameState`))
        (bind _returnvalue (`Controller.K2_GetPawn` (`PlayerState.GetPlayerController` _array_element)))
        (`/Engine/EditorBlueprintResources/StandardMacros.IsValid` _returnvalue :!label _label_4
          (:`Is Valid`
            (bind _asbp_test_character (cast `/Game/_GamePlay/Network/BP_TestCharacter` _returnvalue))
            (`/Game/_GamePlay/Network/BP_TestCharacter.Multicast_InitVOIP` _asbp_test_character))
          (:`Is Not Valid`
            (`KismetSystemLibrary.RetriggerableDelay` 0.2)
            (goto _label_4)))))
    (:`Is Not Valid`
      (`KismetSystemLibrary.RetriggerableDelay` 0.2)
      (goto _label_3))))

(fn `UserConstructionScript`)