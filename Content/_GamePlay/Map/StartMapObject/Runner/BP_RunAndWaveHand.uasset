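; A start-map runner that moves a mesh along a spline on a repeating 14-second loop and toggles a hand-wave state.
; A looping 0.01-second timer started on BeginPlay advances the time, which a float curve remaps to a spline position.
; The mesh follows that location with a vertical offset, taking only the spline's yaw, offset by -90 degrees.
; IsPlayWaveHand turns on from 4.5 to 12.5 seconds of each loop.
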(event `self.ReceiveBeginPlay`
  (`KismetSystemLibrary.K2_SetTimerDelegate` (delegate `SplineMove`) 0.01 true))

(event `SplineMove`
  (bind _output_get (set `self.CurTime` (+ (`self.CurTime`) 0.01)))
  (if (>= (`self.CurTime`) 14.0)
    (set `self.CurTime` 0.0)
    (else
      (bind _returnvalue (`SplineComponent.GetTransformAtTime` (`self.Spline`) (`CurveFloat.GetFloatValue` (`self.SplineCurve`) _output_get) "Local" false false))
      (`SceneComponent.K2_SetRelativeTransform` (`self.Mesh`) (`KismetMathLibrary.MakeTransform` (+ (.location _returnvalue) (0.0 0.0 -90.0)) (`KismetMathLibrary.MakeRotator` 0.0 0.0 (+ (.yaw (.rotation _returnvalue)) -90.0))) false false)
      (if (>= (`self.CurTime`) 12.5)
        (set `self.IsPlayWaveHand` false)
        (elif (and (>= (`self.CurTime`) 4.5) (not (`self.IsPlayWaveHand`)))
          (set `self.IsPlayWaveHand` true))))))

(fn `UserConstructionScript`)