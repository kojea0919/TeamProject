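; Floor 2 runner for the start map that moves its mesh along a spline on a repeating 17-second cycle.
; A looping 0.01-second timer started at BeginPlay advances a clock, which a float curve remaps to spline time at constant velocity.
; The mesh takes the spline's local position and yaw with fixed offsets.
; IsChase is true for the first 10 seconds of each cycle, then false.
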(event `self.ReceiveBeginPlay`
  (`KismetSystemLibrary.K2_SetTimerDelegate` (delegate `SplineMove`) 0.01 true))

(event `SplineMove`
  (`|ExecutionSequence`
    (:`then_0`
      (if (>= (`self.CurTime`) 17.0)
        (set `self.CurTime` 0.0)))
    (:`then_1`
      (bind _output_get (set `self.CurTime` (+ (`self.CurTime`) 0.01)))
      (bind _returnvalue (`SplineComponent.GetTransformAtTime` (`self.Spline`) (`CurveFloat.GetFloatValue` (`self.SplineCurve`) _output_get) "Local" true false))
      (`SceneComponent.K2_SetRelativeTransform` (`self.Mesh`) (`KismetMathLibrary.MakeTransform` (+ (.location _returnvalue) (0.0 0.0 -90.0)) (`KismetMathLibrary.MakeRotator` 0.0 0.0 (+ (.yaw (.rotation _returnvalue)) -90.0))) false false)
      (if (>= (`self.CurTime`) 10.0)
        (set `self.IsChase` false)
        (else
          (set `self.IsChase` true))))))

(fn `UserConstructionScript`)