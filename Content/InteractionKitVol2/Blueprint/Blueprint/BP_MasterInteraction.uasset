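; Base interactable actor for Interaction Kit Vol2, providing shared trigger and interact logic.
; Front, back and general boxes, each with a disable flag, register the actor with an overlapping pawn's BP_InteractKitVol2 component.
; Intearct clears CanInteract and calls Interact.
; BeginPlay caches InteractionMesh's relative transform on authority, and helper events set component relative location or rotation.
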(event `self.ReceiveBeginPlay`
  (bind _interactionmesh (`self.InteractionMesh`))
  ;[1 1 1] Begin play get referance
  (`/Engine/EditorBlueprintResources/ActorMacros.Switch Has Authority`
    (:`Authority`
      (set `self.Relative Location` (`SceneComponent.RelativeLocation` _interactionmesh))
      (set `self.Relative Rotation` (`SceneComponent.RelativeRotation` _interactionmesh)))))

(event `SetCanInteract`
  (params (CanInteract :type Boolean))
  ;[1 1 1] Set Values
  (set `self.CanInteract` CanInteract))

(event `Intearct`
  ;[1 1 1] Initiation of interaction and referencing
  (set `self.CanInteract` false)
  (`/Game/InteractionKitVol2/Blueprint/Interface/BP_Trigger.Interact` self))

(event `self.FrontBox.OnComponentBeginOverlap`
  (params (OverlappedComponent :type "PrimitiveComponent Object Reference") (OtherActor :type "Actor Object Reference") (OtherComp :type "PrimitiveComponent Object Reference") (OtherBodyIndex :type Integer) (bFromSweep :type Boolean) (SweepResult :type "HitResult Structure (by ref)"))
  ;[1 1 1] Box Collisions Begin Overlaps and End Overlaps
  (if (not (`self.DisableFrontBox`))
    (`self.CanInteractOverlap` OtherActor)))

(event `SetRelativeLocationOwning`
  (params (Comp :type "SceneComponent Object Reference") (NewLocation :type "Vector Structure"))
  ;[1 1 1] Set Relative Location - Set Relative Rotation
  (`SceneComponent.K2_SetRelativeLocation` Comp NewLocation false false))

(event `self.BackBox.OnComponentBeginOverlap`
  (params (OverlappedComponent :type "PrimitiveComponent Object Reference") (OtherActor :type "Actor Object Reference") (OtherComp :type "PrimitiveComponent Object Reference") (OtherBodyIndex :type Integer) (bFromSweep :type Boolean) (SweepResult :type "HitResult Structure (by ref)"))
  ;[1 1 1] Box Collisions Begin Overlaps and End Overlaps
  (if (not (`self.DisableBackBox`))
    (`self.CanInteractOverlap` OtherActor)))

(event `SetRelativeRotationOwning`
  (params (Comp :type "SceneComponent Object Reference") (NewRotation :type "Rotator Structure"))
  ;[1 1 1] Set Relative Location - Set Relative Rotation
  (`SceneComponent.K2_SetRelativeRotation` Comp NewRotation false false))

(event `self.GeneralBox.OnComponentBeginOverlap`
  (params (OverlappedComponent :type "PrimitiveComponent Object Reference") (OtherActor :type "Actor Object Reference") (OtherComp :type "PrimitiveComponent Object Reference") (OtherBodyIndex :type Integer) (bFromSweep :type Boolean) (SweepResult :type "HitResult Structure (by ref)"))
  ;[1 1 1] Box Collisions Begin Overlaps and End Overlaps
  (if (not (`self.DisableGeneralBox`))
    (`self.CanInteractOverlap` OtherActor)))

(fn `CanInteractOverlap`
  (params (OtherActor :type "Object Object Reference"))
  (bind _aspawn (cast `Pawn` OtherActor))
  (`/Game/InteractionKitVol2/Blueprint/ActorComponent/BP_InteractKitVol2.SetOverlapCharacter` (`self.GetComponentByClass` _aspawn "/Game/InteractionKitVol2/Blueprint/ActorComponent/BP_InteractKitVol2.BP_InteractKitVol2_C") self))

(fn `UserConstructionScript`)