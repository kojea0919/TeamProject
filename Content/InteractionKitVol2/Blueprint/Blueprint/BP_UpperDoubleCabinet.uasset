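; Interactable upper double cabinet whose two doors swing open and closed in opposite directions.
; Interact calls InteracatMulti, which checks On and plays an Open or Close timeline, lerping InteractionMesh and StaticMesh between their resting rotations and mirrored 90-degree angles.
; BeginPlay caches the StaticMesh resting rotation on authority only.
; When either timeline finishes, authority flips On, calls WhenTheInteractionIsOver and re-enables interaction.
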(event `self.ReceiveBeginPlay`
  ;[1 1 1] Comment
  (`parent.ReceiveBeginPlay`)
  (`/Engine/EditorBlueprintResources/ActorMacros.Switch Has Authority`
    (:`Authority`
      (set `self.Relative Rotation R` (`SceneComponent.RelativeRotation` (`self.StaticMesh`))))))

(event `InteracatMulti`
  ;[1 1 1] Interact
  (if (not (`self.On`))
    (bind (_direction _alpha) (`Timeline|Open` :!via `PlayFromStart`)
      (:`Update`
        (`self.SetRelativeRotationOwning` (`self.InteractionMesh`) (`KismetMathLibrary.RLerp` (`self.Relative Rotation`) (struct :`Yaw` 90.0) _alpha true))
        (`self.SetRelativeRotationOwning` (`self.StaticMesh`) (`KismetMathLibrary.RLerp` (`self.Relative Rotation R`) (struct :`Yaw` -90.0) _alpha true)))
      (:`Finished`
        (`/Engine/EditorBlueprintResources/ActorMacros.Switch Has Authority` :!label _label
          (:`Authority`
            (bind _output_get (set `self.On` (not (`self.On`))))
            (`self.WhenTheInteractionIsOver` _output_get)
            (set `self.CanInteract` true)))))
    (else
      (bind (_direction_2 _alpha_2) (`Timeline|Close` :!via `PlayFromStart`)
        (:`Update`
          (`self.SetRelativeRotationOwning` (`self.InteractionMesh`) (`KismetMathLibrary.RLerp` (struct :`Yaw` 90.0) (`self.Relative Rotation`) _alpha_2 true))
          (`self.SetRelativeRotationOwning` (`self.StaticMesh`) (`KismetMathLibrary.RLerp` (struct :`Yaw` -90.0) (`self.Relative Rotation R`) _alpha_2 true)))
        (:`Finished`
          (goto _label))))))

(event `/Game/InteractionKitVol2/Blueprint/Interface/BP_Trigger.Interact`
  ;[1 1 1] Interact
  (`self.InteracatMulti`))

(fn `UserConstructionScript`
  (`parent.UserConstructionScript`))