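; Interactable storage cabinet, built on a parent interaction class, whose two doors swing open and closed in opposite directions.
; Interact calls InteracatMulti, which plays the Open timeline or reverses the Close timeline according to the On state.
; The timelines lerp the interaction mesh and left door from their stored rotations.
; On completion, the authority flips On, reports the interaction as over and re-enables interaction.
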(event `self.ReceiveBeginPlay`
  ;[1 1 1] Comment
  (`parent.ReceiveBeginPlay`)
  (`/Engine/EditorBlueprintResources/ActorMacros.Switch Has Authority`
    (:`Authority`
      (set `self.Relative Rotation L` (`SceneComponent.RelativeRotation` (`self.SM_StorageCabinetDoorL`))))))

(event `InteracatMulti`
  ;[1 1 1] Interact
  (if (not (`self.On`))
    (bind (_direction _alpha) (`Timeline|Open` :!via `PlayFromStart`)
      (:`Update`
        (`self.SetRelativeRotationOwning` (`self.InteractionMesh`) (`KismetMathLibrary.RLerp` (`self.Relative Rotation`) (struct :`Yaw` 90.0) _alpha true))
        (`self.SetRelativeRotationOwning` (`self.SM_StorageCabinetDoorL`) (`KismetMathLibrary.RLerp` (`self.Relative Rotation L`) (struct :`Yaw` -90.0) _alpha)))
      (:`Finished`
        (`/Engine/EditorBlueprintResources/ActorMacros.Switch Has Authority` :!label _label
          (:`Authority`
            (bind _output_get (set `self.On` (not (`self.On`))))
            (`self.WhenTheInteractionIsOver` _output_get)
            (set `self.CanInteract` true)))))
    (else
      (bind (_direction_2 _alpha_2) (`Timeline|Close` :!via `ReverseFromEnd`)
        (:`Update`
          (`self.SetRelativeRotationOwning` (`self.InteractionMesh`) (`KismetMathLibrary.RLerp` (`self.Relative Rotation`) (struct :`Yaw` 90.0) _alpha_2 true))
          (`self.SetRelativeRotationOwning` (`self.SM_StorageCabinetDoorL`) (`KismetMathLibrary.RLerp` (`self.Relative Rotation L`) (struct :`Yaw` -90.0) _alpha_2)))
        (:`Finished`
          (goto _label))))))

(event `/Game/InteractionKitVol2/Blueprint/Interface/BP_Trigger.Interact`
  ;[1 1 1] Interact
  (`self.InteracatMulti`))

(fn `UserConstructionScript`
  (`parent.UserConstructionScript`))