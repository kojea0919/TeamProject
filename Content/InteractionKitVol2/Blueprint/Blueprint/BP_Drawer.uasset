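; BP_Drawer is an interactable drawer that slides open and closed on interaction.
; Interact calls InteracatMulti, which plays or reverses the OpenAndClose timeline depending on the On flag.
; The timeline lerps InteractionMesh between RelativeLocation and a point 25 units back along X.
; On finish, only the authority flips On, signals that the interaction is over and re-enables CanInteract.
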(event `self.ReceiveBeginPlay`
  (`parent.ReceiveBeginPlay`))

(event `InteracatMulti`
  ;[1 1 1] Interact
  (if (not (`self.On`))
    (bind (_direction _alpha) (`Timeline|OpenAndClose` :!via `PlayFromStart` :!label _label)
      (:`Update`
        (`self.SetRelativeLocationOwning` (`self.InteractionMesh`) (`KismetMathLibrary.VLerp` (`self.Relative Location`) (`KismetMathLibrary.MakeVector` (- (.x (`self.Relative Location`)) 25.0) (.y (`self.Relative Location`)) (.z (`self.Relative Location`))) _alpha)))
      (:`Finished`
        (`/Engine/EditorBlueprintResources/ActorMacros.Switch Has Authority`
          (:`Authority`
            (bind _output_get (set `self.On` (not (`self.On`))))
            (`self.WhenTheInteractionIsOver` _output_get)
            (set `self.CanInteract` true)))))
    (else
      (goto _label :!via `ReverseFromEnd`))))

(event `/Game/InteractionKitVol2/Blueprint/Interface/BP_Trigger.Interact`
  ;[1 1 1] Interact
  (`self.InteracatMulti`))

(fn `UserConstructionScript`
  (`parent.UserConstructionScript`))